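; Gameplay ability for the player's dodge roll, steered by the last movement input.
; After a brief delay, it sets motion warping targets for roll direction and landing point, then plays the roll montage and ends with it.
; The landing point comes from a downward object trace at a level-scaled distance ahead.
; The trace result is used without a hit check, and its debug draw is persistent.
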(event Ability|EventActivateAbility
  (Utilities|FlowControl|Delay 0.05)
  (CallFunction|ComputeRollDirectionandDistance)
  (|PlayMontageandWaitProxy "None" "/Game/PlayerCharacter/Montage/AM_PlayerHero_Roll.AM_PlayerHero_Roll" 1.0 "None" true 1.0 0.0 false
    (:OnCompleted
      _)
    (:OnBlendOut
      _)
    (:OnInterrupted
      _)
    (:OnCancelled
      _))
  (Ability|EndAbility))

(event Ability|EventOnEndAbility
  (params (bWasCancelled :type Boolean)))

(fn ComputeRollDirectionandDistance
  (LocalVariables|SetCachedRollingDirection (Math|Vector|Normalize (Class|Pawn|GetLastMovementInputVector (Class|PlaygroundPlayerGameplayAbility|GetPlayerCharacterfromActorInfo))))
  (Utilities|FlowControl|Sequence
    (:then_0
      ;[0.01846 0.15 0.06857 0.5] Rolling Direction
      (Class|MotionWarpingComponent|AddorUpdateWarpTargetfromLocationandRotation (Variables|/Script/Project_V.PlaygroundBaseCharacter|GetMotionWarpingComponent (Class|PlaygroundPlayerGameplayAbility|GetPlayerCharacterfromActorInfo)) "RollingDirection" "0, 0, 0" (Math|Rotator|MakeRotfromX (LocalVariables|GetCachedRollingDirection))))
    (:then_1
      ;[0.15 0.07091 0.1366 0.5] Rolling Distance
      (bind _outhit (Collision|LineTraceForObjects (+ (Transformation|GetActorLocation (Class|PlaygroundPlayerGameplayAbility|GetPlayerCharacterfromActorInfo)) (* (LocalVariables|GetCachedRollingDirection) (Class|PlaygroundFunctionLibrary|GetScalableFloatValueatLevel (Variables|Default|GetRollingDistanceScalableFloat) (Math|Conversions|ToFloat(Integer) (Ability|GetAbilityLevel))))) (+ (+ (Transformation|GetActorLocation (Class|PlaygroundPlayerGameplayAbility|GetPlayerCharacterfromActorInfo)) (* (LocalVariables|GetCachedRollingDirection) (Class|PlaygroundFunctionLibrary|GetScalableFloatValueatLevel (Variables|Default|GetRollingDistanceScalableFloat) (Math|Conversions|ToFloat(Integer) (Ability|GetAbilityLevel))))) (* (* (Transformation|GetActorUpVector (Class|PlaygroundPlayerGameplayAbility|GetPlayerCharacterfromActorInfo)) -1.0) 5e+02)) (Variables|Default|GetObject%20Types) false 0 "Persistent"))
      (Class|MotionWarpingComponent|AddorUpdateWarpTargetfromLocation (Variables|/Script/Project_V.PlaygroundBaseCharacter|GetMotionWarpingComponent (Class|PlaygroundPlayerGameplayAbility|GetPlayerCharacterfromActorInfo)) "RollTargetLocation" (.ImpactPoint (Collision|BreakHitResult _outhit))))))